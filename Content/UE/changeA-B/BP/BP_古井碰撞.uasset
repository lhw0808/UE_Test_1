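; Ancient well trigger that ends a possessed BP_B's run, awards a soul and returns the player to the original BP_A character.
; On overlap it disables controller input, plays BP_B's jump-down montage and, after a delay, increments the controller's soul count.
; If the original character is valid, it unhides it at its start location, repossesses it, destroys BP_B, clears and resets the countdown, and enables BP_A's input.
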(event `self.ReceiveActorBeginOverlap`
  (params (OtherActor :type "Actor Object Reference"))
  ; 碰撞事件 切換並回到初始點
  (bind _asbp_my_controller (cast `/Game/UE/changeA-B/BP/BP_MyController` (`GameplayStatics.GetPlayerController` 0))) ; 控制中心
  (`self.DisableInput` _asbp_my_controller null) ; 暫停玩家動作
  (bind _asbp_b (cast `/Game/UE/changeA-B/BP/BP_B` OtherActor))
  (`Character.PlayAnimMontage` _asbp_b "/Game/UE/changeA-B/測試村民素材/Jumping_Down__1__Montage.Jumping_Down__1__Montage" 1.0 "None")
  (`KismetSystemLibrary.Delay` 3.0)
  (set `/Game/UE/changeA-B/BP/BP_MyController.靈魂數量` (+ (`/Game/UE/changeA-B/BP/BP_MyController.靈魂數量` _asbp_my_controller) 1) _asbp_my_controller)
  (bind _originalcharacter (`/Game/UE/changeA-B/BP/BP_B.OriginalCharacter` _asbp_b))
  (`/Engine/EditorBlueprintResources/StandardMacros.IsValid` _originalcharacter ; 確認玩家是否存在
    (:`Is Valid`
      (bind _asbp_a (cast `/Game/UE/changeA-B/BP/BP_A` _originalcharacter))
      (`self.SetActorHiddenInGame` _asbp_a false) ; 顯示角色（取消 Hidden）
      (`self.SetActorEnableCollision` _asbp_a true) ; 開啟碰撞
      (`self.K2_SetActorLocation` _originalcharacter (`/Game/UE/changeA-B/BP/BP_A.初始位置` _asbp_a) false false) ; 移動到初始位置
      (`Controller.Possess` (`GameplayStatics.GetPlayerController` 0) _originalcharacter) ; 附身回 A
      (`self.K2_DestroyActor` _asbp_b) ; 刪除BP_B
      (`KismetSystemLibrary.K2_ClearAndInvalidateTimerHandle` (`/Game/UE/changeA-B/BP/BP_A.時間` _asbp_a)) ; 清除倒數
      (set `/Game/UE/changeA-B/BP/BP_A.限制倒數時間` 5.0 _asbp_a) ; 回復倒數時間
      (`self.EnableInput` _asbp_a null) ; 重置
    )))

(fn `UserConstructionScript`)